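; BP_TestFlower is a test Blueprint in the flower logic that reports which tagged static mesh actors overlap its SpawnCollision component.
; A Delay on Tick throttles the check to roughly every three seconds, gathering overlapping StaticMeshActors and keeping those tagged "Minchia".
; Their display names are concatenated without separators, printed as a long-lasting debug string, then cleared for the next pass.
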(event EventBeginPlay
  (|CallParentFunction) ; This node is disabled and will not be called.\nDrag off pins to build functionality.
)

(event Collision|EventActorBeginOverlap
  (params (OtherActor :type Actor%20Object%20Reference))
  (|CallParentFunction OtherActor) ; This node is disabled and will not be called.\nDrag off pins to build functionality.
)

(event EventTick
  (params (DeltaSeconds :type Float%20%28single-precision%29))
  (|CallParentFunction DeltaSeconds)
  (Utilities|FlowControl|Delay 3.0)
  (bind _output_get (Variables|Default|SetOverlapping%20Actors (Collision|GetOverlappingActors (Variables|Default|GetSpawnCollision) "/Script/Engine.StaticMeshActor" :!class /Script/Engine.PrimitiveComponent)))
  (for _array_element _output_get
    (if (Actor|ActorHasTag _array_element "Minchia")
      (Variables|Default|SetIn%20String (Utilities|String|Append (Variables|Default|GetIn%20String) (Utilities|GetDisplayName _array_element)))))
  (Development|PrintString (Variables|Default|GetIn%20String) true true "(R=0.000000,G=0.660000,B=1.000000,A=1.000000)" 5e+01)
  (Variables|Default|SetIn%20String ""))

(fn ConstructionScript
  (|CallParentFunction))