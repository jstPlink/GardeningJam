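; Flower actor that grows, releases pollen, can be fed to clone itself, then dies into the GameMode's object pool.
; A growth timer triggers staggered pollen spawns with random impulses, then opens cloning and starts the death timer.
; Players interact through a trigger range; sufficient Feeding spawns a new flower at a random nearby offset.
; Delay-throttled Tick shows state and remaining time on front and back widgets.
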(event OnComponentBeginOverlap(TriggerRange)
  (params (OverlappedComponent :type Primitive%20Component%20Object%20Reference) (OtherActor :type Actor%20Object%20Reference) (OtherComp :type Primitive%20Component%20Object%20Reference) (OtherBodyIndex :type Integer) (bFromSweep :type Boolean) (SweepResult :type Hit%20Result%20Structure%20%28by%20ref%29))
  ;[1 1 1] PlayerInteraction
  (if (CallFunction|CanPlayerInteract OtherActor)
    (Default|SetInteractableObject (CallFunction|GetPlayer) self)))

(event Custom|Die
  (bind _gamemode (CallFunction|GetGameMode))
  ;[1 1 1] Waiting to die
  (Default|SubtractFlower _gamemode)
  (Variables|Enum|SetState "NewEnumerator3")
  (Default|AddtoPool (Default|GetObjectPool _gamemode) self "NewEnumerator1"))

(event Custom|Spawn%20Polline
  ;[1 1 1] Fertility Status
  (Variables|Enum|SetState "NewEnumerator1")
  (if (<= (Variables|Statistiche|GetNSpawns) 0) :!label _label
    ;[1 1 1] Waiting to die
    (Variables|Statistiche|SetReadyToClone true)
    (bind _returnvalue (Utilities|Time|SetTimerbyEvent (delegate Custom|Die) (Variables|Timer|GetLiveMaxTime)))
    (else
      (Math|Integer|DecrementInt (Variables|Statistiche|GetNSpawns)
        (:%20%20
          (bind _returnvalue_2 (Game|SpawnActorfromClass (Variables|Reference|GetPollineRef) (Transformation|GetWorldTransform (Variables|Default|GetSpawnPosition)) "Undefined" 0 0))
          (bind _asbp_pollen (Utilities|Casting|CastToBP_Pollen _returnvalue_2))
          (Default|Initialize _asbp_pollen)
          (Physics|AddImpulse (Variables|/Game/Blueprints/FlowerLogic/BP_Spawnable.BP_Spawnable_C|GetMesh _asbp_pollen) (CallFunction|GetRndPollineImpulse) "None" false)
          (Utilities|FlowControl|Delay 0.1)
          (goto _label))))))

(event Custom|Initialized
  ;[1 1 1] Birth
  (Variables|Enum|SetState "NewEnumerator0")
  (Default|AddFlower (CallFunction|GetGameMode))
  ;[1 1 1] Growth Status
  (bind _returnvalue (Utilities|Time|SetTimerbyEvent (delegate Custom|Spawn%20Polline) (Variables|Timer|GetGrowthMaxTime))))

(event EventBeginPlay
  ;[1 1 1] Birth
  (Utilities|FlowControl|Sequence
    (:then_0
      (bind _asbpw_flower_description (Utilities|Casting|CastToBPW_FlowerDescription (UserInterface|GetWidget (Variables|Default|GetFrontWidget))))
      (Variables|Reference|SetFlowerDesRef2 _asbpw_flower_description)
      (bind _asbpw_flower_description_2 (Utilities|Casting|CastToBPW_FlowerDescription (UserInterface|GetWidget (Variables|Default|GetBackWidget))))
      (Variables|Reference|SetFlowerDesRef1 _asbpw_flower_description_2))
    (:then_1
      (Variables|Enum|SetState "NewEnumerator0")
      (if (Variables|Tool|GetPlacedInWorld)
        (Default|AddFlower (CallFunction|GetGameMode))
        ;[1 1 1] Growth Status
        (bind _returnvalue (Utilities|Time|SetTimerbyEvent (delegate Custom|Spawn%20Polline) (Variables|Timer|GetGrowthMaxTime)))))))

(event EventTick
  (params (DeltaSeconds :type Float%20%28single-precision%29))
  (bind _state (Variables|Enum|GetState))
  (bind _liveremainingtime (Variables|Timer|GetLiveRemainingTime))
  (bind _returnvalue (Math|Float|Truncate _liveremainingtime))
  ;[1 1 1] Refresh State
  (Utilities|FlowControl|Delay 0.1)
  (Default|RefreshState (Variables|Reference|GetFlowerDesRef1) (Utilities|Select :Index _state :NewEnumerator0 (Math|Float|Truncate (Variables|Timer|GetGrowthRemainingTime)) :NewEnumerator1 _returnvalue :NewEnumerator2 _returnvalue :NewEnumerator3 -1) (Utilities|Text|ToText(String) (Utilities|String|EnumtoString _state))))

(fn ConstructionScript)

(fn SpawnFiore
  (params (Class :type Actor%20Class%20Reference))
  (Game|SpawnActorfromClass Class (Math|Transform|MakeTransform (CallFunction|GetRndFlowerLoc) "0, 0, 0" "1,1,1") "Undefined" 0 0))

(fn Feeding
  (params (FeedNumber :type Integer))
  ;[1 1 1] Player has polline >= than hunger value
  (if (and (>= FeedNumber (Variables|Statistiche|GetHunger)) (Variables|Statistiche|GetReadyToClone))
    (Variables|Statistiche|SetHunger 0)
    (LocalVariables|Settemp (- FeedNumber (Variables|Statistiche|GetHunger)))
    (Variables|Statistiche|SetReadyToClone false)
    (Variables|Enum|SetState "NewEnumerator2")
    (CallFunction|SpawnFiore (Variables|Reference|GetSelfRef))
    (else
      ;[1 1 1] Player has less polline than hunger value
      (LocalVariables|Settemp FeedNumber)))
  (return (LocalVariables|Gettemp)))

(fn GetRndFlowerLoc
  (bind _returnvalue (Transformation|GetActorLocation))
  (bind _maxrange (Variables|Statistiche|GetMaxRange))
  (bind _minrange (Variables|Statistiche|GetMinRange))
  (bind _maxrange_2 (Variables|Statistiche|GetMaxRange))
  (bind _minrange_2 (Variables|Statistiche|GetMinRange))
  (return (Math|Vector|MakeVector (+ (.x _returnvalue) (Math|Conversions|ToFloat(Integer) (Utilities|Select :Index (Math|Random|RandomInteger 2) :Option%200 (Math|Random|RandomIntegerinRange _minrange_2 _maxrange_2) :Option%201 (Math|Random|RandomIntegerinRange (* _maxrange_2 -1) (* _minrange_2 -1))))) (+ (.y _returnvalue) (Math|Conversions|ToFloat(Integer) (Utilities|Select :Index (Math|Random|RandomInteger 2) :Option%200 (Math|Random|RandomIntegerinRange _minrange _maxrange) :Option%201 (Math|Random|RandomIntegerinRange (* _maxrange -1) (* _minrange -1))))) (.z _returnvalue))))

(fn GetRndPollineImpulse
  (bind _maxxyimpulse (Variables|Statistiche|GetMaxXYImpulse))
  (bind _minxyimpulse (Variables|Statistiche|GetMinXYImpulse))
  (bind _maxxyimpulse_2 (Variables|Statistiche|GetMaxXYImpulse))
  (bind _minxyimpulse_2 (Variables|Statistiche|GetMinXYImpulse))
  (return (Math|Vector|MakeVector (Utilities|Select :Index (Math|Random|RandomInteger 2) :Option%200 (Math|Random|RandomFloatinRange (Math|Conversions|ToFloat(Integer) (* _maxxyimpulse_2 0)) (Math|Conversions|ToFloat(Integer) (* _minxyimpulse_2 -1))) :Option%201 (Math|Random|RandomFloatinRange (Math|Conversions|ToFloat(Integer) _minxyimpulse_2) (Math|Conversions|ToFloat(Integer) _maxxyimpulse_2))) (Utilities|Select :Index (Math|Random|RandomInteger 2) :Option%200 (Math|Random|RandomFloatinRange (Math|Conversions|ToFloat(Integer) (* _maxxyimpulse 0)) (Math|Conversions|ToFloat(Integer) (* _minxyimpulse -1))) :Option%201 (Math|Random|RandomFloatinRange (Math|Conversions|ToFloat(Integer) _minxyimpulse) (Math|Conversions|ToFloat(Integer) _maxxyimpulse))) (Math|Random|RandomFloatinRange (Math|Conversions|ToFloat(Integer) (Variables|Statistiche|GetMinZImpulse)) (Math|Conversions|ToFloat(Integer) (Variables|Statistiche|GetMaxZImpulse))))))