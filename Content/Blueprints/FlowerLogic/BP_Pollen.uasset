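; BP_Pollen is a pooled, floating pollen pickup that adds to the player's pollen on overlap.
; Initialize enables physics-only collision, moves the mesh to the actor location and starts Tick.
; Tick applies height-dependent upward force and gradually damps horizontal velocity with a lerp.
; Pickup or a random timeout returns the actor to the object pool and stops Tick.
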(event OnComponentBeginOverlap(Trigger)
  (params (OverlappedComponent :type Primitive%20Component%20Object%20Reference) (OtherActor :type Actor%20Object%20Reference) (OtherComp :type Primitive%20Component%20Object%20Reference) (OtherBodyIndex :type Integer) (bFromSweep :type Boolean) (SweepResult :type Hit%20Result%20Structure%20%28by%20ref%29))
  (if (CallFunction|CanPlayerInteract OtherActor)
    (Default|UpdatePollen (CallFunction|GetPlayer) 1)
    ;[1 1 1] Initial spawnable behavior
    (Default|AddtoPool (CallFunction|GetObjectPool) self "NewEnumerator5")
    (Actor|Tick|SetActorTickEnabled false)))

(event Custom|Initialize
  (bind _mesh (Variables|Character|GetMesh))
  ;[1 1 1] custom start
  (Collision|SetCollisionEnabled _mesh "PhysicsOnly")
  (Transformation|SetWorldLocation _mesh (Transformation|GetActorLocation) false true)
  (Actor|Tick|SetActorTickEnabled true)
  ;[1 1 1] Initial spawnable behavior
  (Utilities|FlowControl|Delay (Math|Random|RandomFloatinRange 15.0 6e+01))
  (Default|AddtoPool (CallFunction|GetObjectPool) self "NewEnumerator5")
  (Actor|Tick|SetActorTickEnabled false))

(event EventBeginPlay
  (Actor|Tick|SetActorTickEnabled false))

(event EventTick
  (params (DeltaSeconds :type Float%20%28single-precision%29))
  (bind _mesh (Variables|Character|GetMesh))
  (bind _mesh_2 (Variables|Character|GetMesh))
  (bind _returnvalue (Transformation|GetWorldLocation _mesh))
  (if (Utilities|Enum|Equal(Enum) (Collision|GetCollisionEnabled (Variables|Character|GetMesh)) "PhysicsOnly")
    ;[1 1 1] floating
    (Physics|AddForce _mesh_2 (Math|Vector|MakeVector 0.0 0.0 (select (< (.z _returnvalue) 5e+02) 1.7e+02 (select (> (.z _returnvalue) 4e+03) 8e+01 1e+02))) "None" false)
    ;[1 1 1] lerp x y movement
    (bind _returnvalue_2 (Physics|GetPhysicsLinearVelocity _mesh_2 "None"))
    (Physics|SetPhysicsLinearVelocity _mesh_2 (Math|Vector|Lerp(Vector) _returnvalue_2 (Math|Vector|MakeVector 0.0 0.0 (.Z (Math|Vector|BreakVector _returnvalue_2))) 0.01) false "None")))

(fn ConstructionScript
  (|CallParentFunction))