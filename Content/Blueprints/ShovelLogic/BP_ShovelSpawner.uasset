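; Shovel spawner that keeps placing shovels around its location at short random intervals throughout play.
; Each wave's count is twice the GameMode's flower count, so difficulty scales linearly.
; Shovels come from an object pool at randomized, vertically offset locations based on Length and Width, then get Setup called.
; The construction script sizes the Box component from those dimensions and draws a debug box.
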(event EventBeginPlay
  ;[1 1 1] Set reference
  (Variables|Default|SetAs%20My%20Game%20Mode (CallFunction|GetGameMode))
  ;[1 1 1] delay random
  (Utilities|FlowControl|Delay (Math|Random|RandomFloatinRange 3.0 6.0) :!label _label)
  ;[1 1 1] Spawn as many shovel as the difficulty of the game
  (bind _numberofshovels (CallFunction|CalculateDifficulty (Default|GetNumberOfFlowers (Variables|Default|GetAs%20My%20Game%20Mode))))
  (for _index (range 1 _numberofshovels)
    (bind _output_get (Variables|Default|SetNewLocation (CallFunction|RandomLocationOfShovel)))
    (bind _objectpooled (Default|GetfromPool (CallFunction|GetObjectPool) "NewEnumerator3" (|RndTransform _output_get)))
    (bind _asbp_shovel (Utilities|Casting|CastToBP_Shovel _objectpooled))
    (Default|Setup _asbp_shovel true))
  (goto _label))

(fn ConstructionScript
  (bind _length (Variables|Default|GetLength))
  (bind _width (Variables|Default|GetWidth))
  (Rendering|Debug|DrawDebugBox :Center (Transformation|GetActorLocation) :Extent (Math|Vector|MakeVector _length _width 1e+01) :Thickness 5.0)
  (Components|Box|SetBoxExtent (Variables|Default|GetBox) (Math|Vector|MakeVector _length _width 2e+01) true))

(fn RandomLocationOfShovel
  (bind _returnvalue (Transformation|GetActorLocation))
  (bind _length (Variables|Default|GetLength))
  (return (Math|Vector|MakeVector (Utilities|Select :Index (Math|Random|RandomInteger 2) :Option%200 (Math|Random|RandomFloatinRange (.x _returnvalue) (+ (.x _returnvalue) _length)) :Option%201 (Math|Random|RandomFloatinRange (- (.x _returnvalue) _length) (.x _returnvalue))) (Utilities|Select :Index (Math|Random|RandomInteger 2) :Option%200 (Math|Random|RandomFloatinRange (.y _returnvalue) 0.0) :Option%201 (Math|Random|RandomFloatinRange (- (.y _returnvalue) (Variables|Default|GetWidth)) (.y _returnvalue))) (- (.z _returnvalue) (Variables|Default|GetVertical%20offset)))))

(fn CalculateDifficulty
  (params (InputNumber :type Integer))
  ;[1 1 1] Per ora è una funzione lineare: numero di rastrelli = numero di fiori per due
  (return (* InputNumber 2)))