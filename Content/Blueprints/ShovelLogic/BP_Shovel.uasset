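; BP_Shovel is a physics-driven shovel that fades out of play after landing, by sinking away and destroying itself.
; When either Mesh or Cube hits a "Ground"-tagged actor, it waits, then disables collision and physics on both and applies a ghost material.
; A slowed timeline then lerps Mesh downward before the actor is destroyed.
; An unconnected teleport node remains from an object-pool fix.
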(event OnComponentHit(Cube)
  (params (HitComponent :type Primitive%20Component%20Object%20Reference) (OtherActor :type Actor%20Object%20Reference) (OtherComp :type Primitive%20Component%20Object%20Reference) (NormalImpulse :type Vector :default "0, 0, 0") (Hit :type Hit%20Result%20Structure%20%28by%20ref%29))
  ;[1 1 1] Bros
  (if (Actor|ActorHasTag OtherActor "Ground")
    (Utilities|FlowControl|Delay (Variables|Default|GetDelay))
    ;;[0 0.07361 1] Disattiva collisioni
    (Collision|SetCollisionEnabled (Variables|Default|GetMesh) "NoCollision")
    (Physics|SetSimulatePhysics (Variables|Default|GetMesh) false)
    (Rendering|Material|SetMaterial (Variables|Default|GetMesh) 0 "/Game/2_Assets/Materials/GhostMaterial.GhostMaterial")
    (CallFunction|Descent)))

(event OnComponentHit(Mesh)
  (params (HitComponent :type Primitive%20Component%20Object%20Reference) (OtherActor :type Actor%20Object%20Reference) (OtherComp :type Primitive%20Component%20Object%20Reference) (NormalImpulse :type Vector :default "0, 0, 0") (Hit :type Hit%20Result%20Structure%20%28by%20ref%29))
  ;[1 1 1] Bros
  (if (Actor|ActorHasTag OtherActor "Ground")
    (Utilities|FlowControl|Delay (Variables|Default|GetDelay))
    ;;[0 0.07361 1] Disattiva collisioni
    (Collision|SetCollisionEnabled (Variables|Default|GetMesh) "NoCollision")
    (Physics|SetSimulatePhysics (Variables|Default|GetMesh) false)
    (Rendering|Material|SetMaterial (Variables|Default|GetMesh) 0 "/Game/2_Assets/Materials/GhostMaterial.GhostMaterial")
    (CallFunction|Descent)))

(event Custom|Descent
  ;[1 1 1] Comment
  (Variables|Default|SetCurrentLocation (Transformation|GetWorldLocation (Variables|Default|GetMesh)))
  (Components|Timeline|SetPlayRate (Variables|Default|GetDescentTimeline) 0.2)
  (bind _descentcurve (Timeline|DescentTimeline Play)
    (:Update
      (Transformation|SetWorldLocation (Variables|Default|GetMesh) (Math|Vector|Lerp(Vector) (Variables|Default|GetCurrentLocation) (Math|Vector|MakeVector (.x (Variables|Default|GetCurrentLocation)) (.y (Variables|Default|GetCurrentLocation)) (- (.z (Variables|Default|GetCurrentLocation)) (Variables|Default|GetDescentNumber))) _descentcurve) false false))
    (:Finished
      (Actor|DestroyActor))))

(event EventBeginPlay
  ;[0 0.07361 1] Comment
  (Physics|SetSimulatePhysics (Variables|Default|GetMesh) true))

(fn ConstructionScript)