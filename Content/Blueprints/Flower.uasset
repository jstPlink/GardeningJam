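; Flower actor that releases pollen (Polline) actors once its growth time has passed.
; BeginPlay sets a timer on SpawnPolline; the fertility and growth status checks exist only as comments.
; SpawnPolline loops over the pollen count, spawning ClassRef at the SpawnCrown transform and giving each Polline mesh a small upward impulse.
; A half-second Delay inside the loop leads to its break.
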(event Custom|Spawn%20Polline
  ;[1 1 1] Fertility Status
  (Utilities|FlowControl|ForLoopwithBreak 0 (Variables|Default|GetNPolline) :!label _label
    (:LoopBody
      (bind _returnvalue (Game|SpawnActorfromClass (Variables|Default|GetClassRef) (Transformation|GetWorldTransform (Variables|Default|GetSpawnCrown)) "Undefined" 0 0))
      (bind _aspolline (Utilities|Casting|CastToPolline _returnvalue))
      (Physics|AddImpulse (Variables|/Game/Blueprints/Polline.Polline_C|GetMesh _aspolline) "0, 0,20.000000" "None" false)
      (Utilities|FlowControl|Delay 0.5)
      (goto _label Break))))

(event EventBeginPlay
  ;[1 1 1] Initial checks
  ;[1 1 1] Growth Status
  (Utilities|Time|SetTimerbyEvent (delegate Custom|Spawn%20Polline) (Variables|Default|GetGrowthTime)))

(fn ConstructionScript)