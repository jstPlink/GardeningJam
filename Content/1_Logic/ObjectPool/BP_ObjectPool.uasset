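; Actor object pool that pre-spawns configured amounts of each object type at BeginPlay and hands them out on request.
; Pooled actors wait at PoolRoot, hidden and without collision; GetFromPool teleports one to the requested transform and re-enables it.
; Storage spans five size-capped actor-to-type maps, tried in order for adding and searching.
; When none holds the requested type, GrowPool spawns GrowAmount more and the request retries.
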(event EventBeginPlay
  (Tool|StartPool))

(fn ConstructionScript)

(fn StartPool
  (bind _keys (Utilities|Map|Keys (Variables|Main|GetObjectToClass)))
  (for _array_element _keys
    (Variables|Tools|SetCurObject _array_element)
    (Tool|GrowPool false)))

(fn AddtoPool
  (params (Actor :type Actor%20Object%20Reference) (Type :type BPE_ObjectPool%20Enum :default "NewEnumerator3"))
  (bind _output_get (Variables|Tools|SetCurActor Actor))
  (Variables|Tools|SetCurObject Type)
  (Tool|ShowObject false _output_get (Transformation|GetRelativeTransform (Variables|Default|GetPoolRoot)))
  (Utilities|AddtoSomePool (Variables|Pools|GetPool1)
    (:NotAdded
      (Utilities|AddtoSomePool (Variables|Pools|GetPool2)
        (:NotAdded
          (Utilities|AddtoSomePool (Variables|Pools|GetPool3)
            (:NotAdded
              (Utilities|AddtoSomePool (Variables|Pools|GetPool4)
                (:NotAdded
                  (Utilities|AddtoSomePool (Variables|Pools|GetPool5)
                    (:NotAdded
                      (Development|PrintString "No more space (Object pool)" true true "(R=1.000000,G=0.000000,B=0.000000,A=1.000000)" 5.0))))))))))))

(fn GetfromPool
  (params (Object :type BPE_ObjectPool%20Enum :default "NewEnumerator3") (NewTransform :type Transform))
  (bind _curactor (Variables|Tools|GetCurActor))
  (Variables|Tools|SetCurObject Object)
  (Variables|Tools|SetNew%20Transform NewTransform)
  (Utilities|SearchObject (Variables|Pools|GetPool1)
    (:Found
      (Utilities|IsValid _curactor :!label _label
        (:Is%20Valid
          (Tool|ShowObject true _curactor (Variables|Tools|GetNew%20Transform))
          (return _curactor))
        (:Is%20Not%20Valid
          (Development|PrintString "Requested object not valid (Object pool)" true true "(R=1.000000,G=0.000000,B=0.000000,A=1.000000)" 5.0))))
    (:Not%20Found
      (Utilities|SearchObject (Variables|Pools|GetPool2)
        (:Found
          (goto _label))
        (:Not%20Found
          (Utilities|SearchObject (Variables|Pools|GetPool3)
            (:Found
              (goto _label))
            (:Not%20Found
              (Utilities|SearchObject (Variables|Pools|GetPool4)
                (:Found
                  (goto _label))
                (:Not%20Found
                  (Utilities|SearchObject (Variables|Pools|GetPool5)
                    (:Found
                      (goto _label))
                    (:Not%20Found
                      (Tool|GrowPool true)
                      (Main|GetfromPool (Variables|Tools|GetCurObject) NewTransform))))))))))))

(fn ShowObject
  (params (Show :type Boolean) (Actor :type Actor%20Object%20Reference) (NewTransform :type Transform))
  (bind (_location _rotation) (Math|Transform|BreakTransform NewTransform))
  (Transformation|Teleport Actor _location _rotation)
  (Rendering|SetActorHiddenInGame Actor (not Show))
  (Collision|SetActorEnableCollision Actor Show)
  (return))

(fn GrowPool
  (params (Grow :type Boolean))
  (bind _objecttoclass (Variables|Main|GetObjectToClass))
  (bind _keys (Utilities|Map|Keys _objecttoclass))
  (bind _values (Utilities|Map|Values _objecttoclass))
  (bind _values_2 (Utilities|Map|Values (Variables|Main|GetObjectToAmount)))
  (for _index (range 0 (- (select Grow (Variables|Main|GetGrowAmount) (Utilities|Array|Get(acopy) _values_2 (Utilities|Array|FindItem _keys (Variables|Tools|GetCurObject)))) 1))
    (bind _returnvalue (Game|SpawnActorfromClass (Utilities|Array|Get(acopy) _values (Utilities|Array|FindItem _keys (Variables|Tools|GetCurObject))) (Transformation|GetRelativeTransform (Variables|Default|GetPoolRoot)) "Undefined" 0 0))
    (Utilities|IsValid _returnvalue
      (:Is%20Valid
        (Main|AddtoPool _returnvalue (Variables|Tools|GetCurObject)))
      (:Is%20Not%20Valid
        (Development|PrintString "Class to spawn not valid (Object pool)" true true "(R=1.000000,G=0.000000,B=0.000000,A=1.000000)" 5.0)
        (return))))
  (return))