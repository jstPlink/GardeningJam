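; Player pawn that flies a physics Sphere on forward, strafe and vertical axes, with a held boost.
; Tick lerps the Sphere's linear velocity toward the input, while Rotate zeroes rotation and damps spin, leaving look and roll inputs unused.
; Sphere hits deal fixed damage, throttled by DoOnce and a retriggerable delay, and broadcast the health ratio.
; Interact only sets a flag; its handling logic is disconnected.
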(event OnComponentHit(Sphere)
  (params (HitComponent :type Primitive%20Component%20Object%20Reference) (OtherActor :type Actor%20Object%20Reference) (OtherComp :type Primitive%20Component%20Object%20Reference) (NormalImpulse :type Vector :default "0, 0, 0") (Hit :type Hit%20Result%20Structure%20%28by%20ref%29))
  ;[1 1 1] collision
  (Utilities|FlowControl|DoOnce false :!label _label
    (:Completed
      (CallFunction|DamagePlayer 8)
      (Utilities|FlowControl|RetriggerableDelay 1.0)
      (goto _label Reset))))

(event EventBeginPlay
  (Variables|Main|SetMaxSpeed (* 1000 (Variables|Main|GetMaxSpeed)))
  (Variables|Default|SetCurHealth (Variables|Main|GetMaxHealth))
  (Default|CallOnHealthUpdate 1.0))

(event Collision|EventActorBeginOverlap
  (params (OtherActor :type Actor%20Object%20Reference)))

(event EventTick
  (params (DeltaSeconds :type Float%20%28single-precision%29))
  (CallFunction|Move)
  (CallFunction|Rotate))

(event Input|ActionEvents|InputActionMovement_Boost
  (params (Key :type Key%20Structure))
  ;[1 1 1] boost
  (:Pressed
    (Variables|Code|SetIsBoosting true))
  (:Released
    (Variables|Code|SetIsBoosting false)))

(event Input|ActionEvents|InputActionInteract
  (params (Key :type Key%20Structure))
  (:Pressed
    (Variables|Code|SetIsInteracting true)))

(event Input|AxisEvents|InputAxisMovement_Forward
  (params (AxisValue :type Float%20%28single-precision%29))
  ;[1 1 1] mov fwd
  (Variables|Code|SetCurFwdMov (* AxisValue (Variables|Main|GetMaxSpeed) (select (Variables|Code|GetIsBoosting) (Variables|Default|GetSpeedMultiplier) 1.0))))

(event Input|AxisEvents|InputAxisMovement_Horizontal
  (params (AxisValue :type Float%20%28single-precision%29))
  ;[1 1 1] mov hor
  (Variables|Code|SetCurHorMov (* AxisValue (Variables|Main|GetMaxSpeed) (select (Variables|Code|GetIsBoosting) (Variables|Default|GetSpeedMultiplier) 1.0))))

(event Input|AxisEvents|InputAxisCamera_Vertical
  (params (AxisValue :type Float%20%28single-precision%29))
  ;[1 1 1] rotationm
  (Variables|Code|SetCurRotPitch (* AxisValue (Variables|Main|GetMaxRotSpeed) (Utilities|Time|GetWorldDeltaSeconds))))

(event Input|AxisEvents|InputAxisCamera_Horizontal
  (params (AxisValue :type Float%20%28single-precision%29))
  ;[1 1 1] rotationm
  (Variables|Code|SetCurRotYaw (* AxisValue (Variables|Main|GetMaxRotSpeed) (Utilities|Time|GetWorldDeltaSeconds))))

(event Input|AxisEvents|InputAxisMovement_Roll
  (params (AxisValue :type Float%20%28single-precision%29))
  ;[1 1 1] rotationm
  (Variables|Code|SetCurRotRoll (* AxisValue (Variables|Main|GetMaxRotSpeed) (Utilities|Time|GetWorldDeltaSeconds) 3.0)))

(event Input|AxisEvents|InputAxisMovement_Up
  (params (AxisValue :type Float%20%28single-precision%29))
  ;[1 1 1] up downù
  (Variables|Code|SetCurUpMov (* AxisValue (Variables|Main|GetMaxSpeed) (select (Variables|Code|GetIsBoosting) (Variables|Default|GetSpeedMultiplier) 1.0) 0.7)))

(fn ConstructionScript)

(fn Move
  (bind _maxspeed (Variables|Main|GetMaxSpeed))
  (bind _isboosting (Variables|Code|GetIsBoosting))
  (bind _speedmultiplier (Variables|Default|GetSpeedMultiplier))
  (bind _sphere (Variables|Default|GetSphere))
  (bind _sphere_2 (Variables|Default|GetSphere))
  (bind _returnvalue (* _maxspeed _speedmultiplier))
  (bind _returnvalue_2 (select _isboosting _returnvalue _maxspeed))
  (bind _returnvalue_3 (Physics|GetPhysicsLinearVelocity _sphere "None"))
  (Physics|SetPhysicsLinearVelocity _sphere (Math|Vector|Lerp(Vector) _returnvalue_3 (+ (* (Math|Vector|GetForwardVector _sphere_2) (Math|Conversions|ToVector(Float) (* (Math|Float|Clamp(Float) (Variables|Code|GetCurFwdMov) (* -1 _returnvalue_2) _returnvalue_2) (Utilities|Time|GetWorldDeltaSeconds)))) (* (Math|Vector|GetRightVector _sphere_2) (Math|Conversions|ToVector(Float) (* (Math|Float|Clamp(Float) (Variables|Code|GetCurHorMov) (* -1 _returnvalue_2) _returnvalue_2) (Utilities|Time|GetWorldDeltaSeconds)))) (* (Math|Vector|GetUpVector _sphere_2) (Math|Conversions|ToVector(Float) (* (Math|Float|Clamp(Float) (Variables|Code|GetCurUpMov) (* -1 _returnvalue_2) _returnvalue_2) (Utilities|Time|GetWorldDeltaSeconds))))) 0.1) false "None"))

(fn Rotate
  (bind _sphere (Variables|Default|GetSphere))
  (Transformation|SetRelativeRotation _sphere (Math|Rotator|MakeRotator 0.0 0.0 0.0) false false)
  (Class|PrimitiveComponent|SetPhysicsAngularVelocityinDegrees _sphere (Math|Vector|Lerp(Vector) (Physics|GetPhysicsAngularVelocityinDegrees _sphere "None") "0, 0, 0" 0.1) false "None"))

(fn DamagePlayer
  (params (Amount :type Integer))
  (Variables|Default|SetCurHealth (- (Variables|Default|GetCurHealth) Amount))
  (Default|CallOnHealthUpdate (/ (Math|Conversions|ToFloat(Integer) (Variables|Default|GetCurHealth)) (Math|Conversions|ToFloat(Integer) (Variables|Main|GetMaxHealth)))))